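; Main player character Blueprint that shows a crosshair and adds look-driven weapon sway.
; BeginPlay creates the WB_Crosshair widget and adds it to the viewport.
; Every Tick, WeaponSway offsets InitRot by look input plus MaxSwayDegree, inverting pitch, and eases the Mock component's relative rotation toward it with RInterpTo.
; MaxSwayDegree acts as an additive offset rather than a limit, as the clamp nodes are unconnected.
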(event EventBeginPlay
  (bind _returnvalue (UserInterface|CreateWidget "/Game/Assets/Widgets/WB_Crosshair.WB_Crosshair_C"))
  (UserInterface|Viewport|AddtoViewport _returnvalue 0))

(event Collision|EventActorBeginOverlap
  (params (OtherActor :type Actor%20Object%20Reference)))

(event EventTick
  (params (DeltaSeconds :type Float%20%28single-precision%29))
  (CallFunction|WeaponSway DeltaSeconds))

(fn ConstructionScript)

(fn WeaponSway
  (params (Delta%20Time :type Float%20%28double-precision%29))
  (bind _returnvalue (Input|EnhancedActionValues|GetIA_Look))
  (bind _maxswaydegree (LocalVariables|GetmaxSwayDegree))
  (bind _initrot (LocalVariables|GetInitRot))
  (bind (_x _y) (Math|Vector2D|BreakVector2D _returnvalue))
  (bind _returnvalue_2 (+ _x _maxswaydegree))
  (LocalVariables|SetFinalRot (Math|Rotator|MakeRotator _returnvalue_2 (+ _y _maxswaydegree) _returnvalue_2))
  (Transformation|SetRelativeRotation (Variables|Default|GetMock) (Math|Interpolation|RInterpTo (Variables|/Script/Engine.SceneComponent|GetRelativeRotation (Variables|Default|GetMock)) (Math|Rotator|MakeRotator (+ (.roll _initrot) (.roll (LocalVariables|GetFinalRot))) (- (.pitch _initrot) (.pitch (LocalVariables|GetFinalRot))) (+ (.yaw _initrot) (.yaw (LocalVariables|GetFinalRot)))) Delta%20Time 5.0) false false))