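; Door control panel Blueprint that shows a prompt widget while something overlaps its box and drives the level's BP_Door.
; On BeginPlay it creates the WB_Door widget and finds the door actor; overlap begin and end toggle the widget's visibility.
; OpenDoor runs only while the widget is visible, gated by a DoOnce.
; One timeline moves the door vertically, then after a delay a second moves it again and resets the gate.
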(event OnComponentBeginOverlap(Box)
  (params (OverlappedComponent :type Primitive%20Component%20Object%20Reference) (OtherActor :type Actor%20Object%20Reference) (OtherComp :type Primitive%20Component%20Object%20Reference) (OtherBodyIndex :type Integer) (bFromSweep :type Boolean) (SweepResult :type Hit%20Result%20Structure%20%28by%20ref%29))
  (Widget|SetVisibility (Variables|Default|GetButonWigRef) "Visible"))

(event OnComponentEndOverlap(Box)
  (params (OverlappedComponent :type Primitive%20Component%20Object%20Reference) (OtherActor :type Actor%20Object%20Reference) (OtherComp :type Primitive%20Component%20Object%20Reference) (OtherBodyIndex :type Integer))
  (Widget|SetVisibility (Variables|Default|GetButonWigRef) "Hidden"))

(event Custom|Open%20Door
  (if (Widget|IsVisible (Variables|Default|GetButonWigRef))
    (Utilities|FlowControl|DoOnce false :!label _label
      (:Completed
        (bind _float_value (Timeline|Timeline Play)
          (:Update
            (Transformation|SetRelativeLocation (Variables|/Game/Assets/BP_Door.BP_Door_C|GetDoor (Variables|Default|GetDoorBpRef)) (Math|Vector|MakeVector 0.0 0.0 (Math|Float|Lerp 0.0 467.0 _float_value)) false false)
            (Utilities|FlowControl|Delay 2.0)
            (bind _float_value_2 (Timeline|Timeline_0 Play)
              (:Update
                (Transformation|SetRelativeLocation (Variables|/Game/Assets/BP_Door.BP_Door_C|GetDoor (Variables|Default|GetDoorBpRef)) (Math|Vector|MakeVector 0.0 0.0 (Math|Float|Lerp 0.0 467.0 _float_value_2)) false false)
                (goto _label Reset)))))))))

(event EventBeginPlay
  (bind _returnvalue (UserInterface|CreateWidget "/Game/Assets/WB_Door.WB_Door_C"))
  (bind _output_get (Variables|Default|SetButonWigRef _returnvalue))
  (UserInterface|Viewport|AddtoViewport _output_get 0)
  (bind _returnvalue_2 (Actor|GetActorOfClass "/Game/Assets/BP_Door.BP_Door_C"))
  (Variables|Default|SetDoorBpRef _returnvalue_2))

(fn ConstructionScript)