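; Rifle weapon Blueprint that applies camera recoil while firing and recovers the aim when firing stops.
; The RecoilTM timeline feeds pitch and yaw curves into player controller input, then reverses at higher speed with negated, amplified values.
; DoOnce gates capture control rotation at fire start and recovery start.
; Their pitch difference scales recovery around RecoilMaxThres, tapering for larger deviations, and the gates reset when the reverse finishes.
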(event Custom|CE_ResetRecoil
  (Utilities|FlowControl|Sequence
    (:then_0
      (Utilities|FlowControl|DoOnce false) ; enters at Reset
    )
    (:then_1
      (Utilities|FlowControl|DoOnce false) ; enters at Reset
    )))

(event EventBeginPlay)

(event Collision|EventActorBeginOverlap
  (params (OtherActor :type Actor%20Object%20Reference)))

(event EventTick
  (params (DeltaSeconds :type Float%20%28single-precision%29)))

(event EventWeaponIsFiring
  (bind _recoilmaxthres (Variables|Default|GetRecoilMaxThres))
  (Components|Timeline|SetPlayRate (Variables|Default|GetRecoilTM) 1.0)
  (Utilities|FlowControl|Sequence
    (:then_0
      (Utilities|FlowControl|DoOnce false
        (:Completed
          (Variables|Default|SetOriginalWeaponRotation (Pawn|GetControlRotation (Game|GetPlayerController 0) :!class /Script/Engine.Controller)))))
    (:then_1
      (bind (_direction _pitch _yaw) (Timeline|RecoilTM Play)
        (:Update
          (switch Utilities|FlowControl|Switch|SwitchonETimelineDirection _direction
            (:Forward
              (CallFunction|UdpdateRecoilPY _pitch _yaw))
            (:Backward
              (Utilities|FlowControl|Sequence
                (:then_0
                  (Utilities|FlowControl|DoOnce false
                    (:Completed
                      (Variables|Default|SetPostRecoil (Pawn|GetControlRotation (Game|GetPlayerController 0) :!class /Script/Engine.Controller)))))
                (:then_1
                  (CallFunction|UdpdateRecoilPY (* _pitch -13.0 (select (> (Math|Float|Absolute(Float) (.Pitch (Math|Rotator|BreakRotator (Math|Rotator|Delta(Rotator) (Variables|Default|GetOriginalWeaponRotation) (Variables|Default|GetPostRecoil))))) _recoilmaxthres) (Math|Float|MapRangeClamped (Math|Float|Absolute(Float) (.Pitch (Math|Rotator|BreakRotator (Math|Rotator|Delta(Rotator) (Variables|Default|GetOriginalWeaponRotation) (Variables|Default|GetPostRecoil))))) (Variables|Default|GetRecoilMaxThres) 3e+01 1.0 0.0) (Math|Float|MapRangeClamped (Math|Float|Absolute(Float) (.Pitch (Math|Rotator|BreakRotator (Math|Rotator|Delta(Rotator) (Variables|Default|GetOriginalWeaponRotation) (Variables|Default|GetPostRecoil))))) 0.0 _recoilmaxthres 0.0 1.0))) (* _yaw -3.0 (select (> (Math|Float|Absolute(Float) (.Pitch (Math|Rotator|BreakRotator (Math|Rotator|Delta(Rotator) (Variables|Default|GetOriginalWeaponRotation) (Variables|Default|GetPostRecoil))))) _recoilmaxthres) (Math|Float|MapRangeClamped (Math|Float|Absolute(Float) (.Pitch (Math|Rotator|BreakRotator (Math|Rotator|Delta(Rotator) (Variables|Default|GetOriginalWeaponRotation) (Variables|Default|GetPostRecoil))))) (Variables|Default|GetRecoilMaxThres) 3e+01 1.0 0.0) (Math|Float|MapRangeClamped (Math|Float|Absolute(Float) (.Pitch (Math|Rotator|BreakRotator (Math|Rotator|Delta(Rotator) (Variables|Default|GetOriginalWeaponRotation) (Variables|Default|GetPostRecoil))))) 0.0 _recoilmaxthres 0.0 1.0)))))))))
        (:Finished
          (switch Utilities|FlowControl|Switch|SwitchonETimelineDirection _direction
            (:Backward
              (CallFunction|CEResetRecoil))))))))

(event EventWeaponStopsFiring
  (bind _recoilmaxthres (Variables|Default|GetRecoilMaxThres))
  (Components|Timeline|SetPlayRate (Variables|Default|GetRecoilTM) 13.0)
  (bind (_direction _pitch _yaw) (Timeline|RecoilTM Reverse)
    (:Update
      (switch Utilities|FlowControl|Switch|SwitchonETimelineDirection _direction
        (:Forward
          (CallFunction|UdpdateRecoilPY _pitch _yaw))
        (:Backward
          (Utilities|FlowControl|Sequence
            (:then_0
              (Utilities|FlowControl|DoOnce false
                (:Completed
                  (Variables|Default|SetPostRecoil (Pawn|GetControlRotation (Game|GetPlayerController 0) :!class /Script/Engine.Controller)))))
            (:then_1
              (CallFunction|UdpdateRecoilPY (* _pitch -13.0 (select (> (Math|Float|Absolute(Float) (.Pitch (Math|Rotator|BreakRotator (Math|Rotator|Delta(Rotator) (Variables|Default|GetOriginalWeaponRotation) (Variables|Default|GetPostRecoil))))) _recoilmaxthres) (Math|Float|MapRangeClamped (Math|Float|Absolute(Float) (.Pitch (Math|Rotator|BreakRotator (Math|Rotator|Delta(Rotator) (Variables|Default|GetOriginalWeaponRotation) (Variables|Default|GetPostRecoil))))) (Variables|Default|GetRecoilMaxThres) 3e+01 1.0 0.0) (Math|Float|MapRangeClamped (Math|Float|Absolute(Float) (.Pitch (Math|Rotator|BreakRotator (Math|Rotator|Delta(Rotator) (Variables|Default|GetOriginalWeaponRotation) (Variables|Default|GetPostRecoil))))) 0.0 _recoilmaxthres 0.0 1.0))) (* _yaw -3.0 (select (> (Math|Float|Absolute(Float) (.Pitch (Math|Rotator|BreakRotator (Math|Rotator|Delta(Rotator) (Variables|Default|GetOriginalWeaponRotation) (Variables|Default|GetPostRecoil))))) _recoilmaxthres) (Math|Float|MapRangeClamped (Math|Float|Absolute(Float) (.Pitch (Math|Rotator|BreakRotator (Math|Rotator|Delta(Rotator) (Variables|Default|GetOriginalWeaponRotation) (Variables|Default|GetPostRecoil))))) (Variables|Default|GetRecoilMaxThres) 3e+01 1.0 0.0) (Math|Float|MapRangeClamped (Math|Float|Absolute(Float) (.Pitch (Math|Rotator|BreakRotator (Math|Rotator|Delta(Rotator) (Variables|Default|GetOriginalWeaponRotation) (Variables|Default|GetPostRecoil))))) 0.0 _recoilmaxthres 0.0 1.0)))))))))
    (:Finished
      (switch Utilities|FlowControl|Switch|SwitchonETimelineDirection _direction
        (:Backward
          (CallFunction|CEResetRecoil))))))

(fn ConstructionScript)

(fn UdpdateRecoilPY
  (params (Val :type Float%20%28single-precision%29) (Val2 :type Float%20%28single-precision%29))
  (bind _returnvalue (Game|GetPlayerController 0))
  (Class|PlayerController|AddPitchInput _returnvalue Val)
  (Class|PlayerController|AddYawInput _returnvalue Val2))